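; A pickaxe tool pickup that spins in the world until a FirstPersonCharacter overlaps its box, then attaches to that character's GripPoint socket as their tool.
; While mining, a DoOnce-gated timeline swings the mesh, and on finish it mines an in-range ores target and loses durability.
; A second timeline plays in reverse to recover and re-arm the swing.
; At zero durability it destroys itself and clears the character's IsPicked flag.
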(event `self.Box.OnComponentBeginOverlap`
  (params (OverlappedComponent :type "PrimitiveComponent Object Reference") (OtherActor :type "Actor Object Reference") (OtherComp :type "PrimitiveComponent Object Reference") (OtherBodyIndex :type Integer) (bFromSweep :type Boolean) (SweepResult :type "HitResult Structure (by ref)"))
  (bind _asfirst_person_character (cast `/Game/_FinalAssets/Blueprints/JunHao/FirstPersonCharacter` OtherActor))
  (set `/Game/_FinalAssets/Blueprints/JunHao/FirstPersonCharacter.isPicked?` true _asfirst_person_character)
  (set `self.picked` true)
  (set `/Game/_FinalAssets/Blueprints/JunHao/FirstPersonCharacter.Tools` self _asfirst_person_character)
  (`self.K2_AttachToComponent` self (`FP_FirstPersonCharacter.Mesh1P` _asfirst_person_character) "GripPoint" "SnapToTarget" "SnapToTarget" "SnapToTarget" true))

(event `self.ReceiveTick`
  (params (DeltaSeconds :type "Float (single-precision)"))
  (bind _distance (`self.Distance`))
  (if (`self.picked`)
    (if (`self.isMining?`)
      (`/Engine/EditorBlueprintResources/StandardMacros.DoOnce` false :!label _label
        (:`Completed`
          (bind (_direction _newtrack_0) (`Timeline|Timeline_0` :!via `PlayFromStart`)
            (:`Update`
              (`SceneComponent.K2_SetRelativeRotation` (`self.PickerMesh`) (`KismetMathLibrary.MakeRotator` 0.0 _newtrack_0) false false))
            (:`Finished`
              (if (`KismetSystemLibrary.IsValid` (`self.MineTarget`))
                (if (and (<= _distance (`self.ToolRange`)) (!= _distance 0.0))
                  (bind _asores (cast `/Game/_FinalAssets/Blueprints/JunHao/ores` (`self.MineTarget`))
                    (:`then`
                      (set `self.Durability` (- (`self.Durability`) 5.0))
                      (`/Game/_FinalAssets/Blueprints/JunHao/ores.Mine` _asores)
                      (if (<= (`self.Durability`) 0.0)
                        (`self.K2_DestroyActor`)
                        (set `/Game/_FinalAssets/Blueprints/JunHao/FirstPersonCharacter.isPicked?` false (`self.Character`))
                        (else
                          (bind (_direction_2 _newtrack_0_2) (`Timeline|Timeline_1` :!via `ReverseFromEnd` :!label _label_2)
                            (:`Update`
                              (`SceneComponent.K2_SetRelativeRotation` (`self.PickerMesh`) (`KismetMathLibrary.MakeRotator` 0.0 _newtrack_0_2) false false))
                            (:`Finished`
                              (goto _label :!via `Reset`))))))
                    (:`CastFailed`
                      (goto _label_2 :!via `ReverseFromEnd`)))
                  (else
                    (goto _label_2 :!via `ReverseFromEnd`)))
                (else
                  (goto _label_2 :!via `ReverseFromEnd`))))))))
    (else
      (`self.K2_AddActorLocalRotation` (struct :`Yaw` 1.0)))))

(fn `UserConstructionScript`)