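; A choppable actor that turns a configurable static mesh into a procedural mesh, apparently for slicing, and limits how many slices it takes.
; The construction script applies the mesh, material and scale to the static mesh component, then copies it into the procedural mesh with collision.
; AddSlice increments a counter and destroys the actor at the slice limit; the cutting itself is not done here.
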(event `AddSlice`
  (bind _result (`/Engine/EditorBlueprintResources/StandardMacros.IncrementInt` (`self.CurrentSlice`))
    (:`  `
      (if (>= _result (`self.MaxSlice`))
        (`self.K2_DestroyActor`)))))

(fn `UserConstructionScript`
  (bind _staticmesh (`self.StaticMesh`))
  (`StaticMeshComponent.SetStaticMesh` _staticmesh (`self.Mesh`))
  (`PrimitiveComponent.SetMaterial` _staticmesh 0 (`self.Material`))
  (`SceneComponent.SetWorldScale3D` _staticmesh (`self.Scale`))
  (`KismetProceduralMeshLibrary.CopyProceduralMeshFromStaticMeshComponent` (`self.StaticMesh`) 0 (`self.ProceduralMesh`) true))