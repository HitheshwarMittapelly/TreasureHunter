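; BrickSpawner is an actor that builds a 3D grid of Brick actors when play begins.
; Three nested loops spawn each Brick at an offset from the spawner's location, scaled by a fixed per-axis spacing.
; Each Brick receives its grid coordinate as an Index vector, which is also added to BrickArray.
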(event `self.ReceiveBeginPlay`
  (for _index (range 3)
    (for _index_2 (range 5)
      (for _index_3 (range 5)
        (bind _returnvalue (`KismetMathLibrary.MakeVector` (`KismetMathLibrary.Conv_IntToDouble` _index) (`KismetMathLibrary.Conv_IntToDouble` _index_2) (`KismetMathLibrary.Conv_IntToDouble` _index_3)))
        (bind _returnvalue_2 (`|SpawnActorFromClass` "/Game/_FinalAssets/Blueprints/Spencer/Brick.Brick_C" (`KismetMathLibrary.Conv_VectorToTransform` (+ (+ (`self.K2_GetActorLocation`) (0.0 40.0 50.0)) (* _returnvalue (15.0 80.0 100.0)))) "Undefined" "OverrideRootScale" null null))
        (bind _output_get (set `/Game/_FinalAssets/Blueprints/Spencer/Brick.Index` _returnvalue _returnvalue_2))
        (`BlueprintMapLibrary.Map_Add` (`self.BrickArray`) null _output_get)))))

(fn `UserConstructionScript`)