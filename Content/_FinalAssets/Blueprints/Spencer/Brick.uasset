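; Brick actor that the player can highlight by looking at it and then destroy.
; PlayerLookAt raises a flag that Tick reads and clears each frame, so the highlight lasts only while the call keeps repeating.
; Tick swaps the cube between brick and arrow materials and sets the activated state to match.
; PlayerRequireDestory destroys the actor only while it is activated.
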(event `PlayerLookAt`
  (set `self.lookAt` true))

(event `self.ReceiveTick`
  (params (DeltaSeconds :type "Float (single-precision)"))
  (bind _brickcube (`self.BrickCube`))
  (if (`self.lookAt`)
    (`PrimitiveComponent.SetMaterial` _brickcube 0 "/Engine/VREditor/UI/ArrowMaterial.ArrowMaterial")
    (set `self.brickActivated` true)
    (else
      (`PrimitiveComponent.SetMaterial` _brickcube 0 "/Game/_FinalAssets/Materials/BrickMaterial.BrickMaterial")
      (set `self.brickActivated` false)))
  (set `self.lookAt` false))

(event `PlayerRequireDestory`
  (if (`self.brickActivated`)
    (`self.K2_DestroyActor`)))

(fn `UserConstructionScript`)